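; Game mode that drives a stress mechanic by spawning entities as stress builds.
; At BeginPlay it caches tagged spawn locations and starts a looping timer to raise stress.
; While stress is positive, IncreaseStress picks a random cached point, ignoring player position, and spawns BP_Entity with a random mesh; only one variant faces the player.
; ChangeStressLevel dispatches to four level handlers, which all currently just destroy spawned entities.
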(event `self.ReceiveBeginPlay`
  (bind _outactors (`GameplayStatics.GetAllActorsWithTag` "EntitySpawnLocation"))
  (for _array_element _outactors
    (`KismetArrayLibrary.Array_Add` (`self.PossibleSpawnLocations`) (`self.K2_GetActorLocation` _array_element)))
  (`KismetSystemLibrary.K2_SetTimerDelegate` (delegate `IncreaseStress`) (`self.StressIncreaseTimeInterval`) true false 1.0))

(event `IncreaseStress`
  (bind _output_get (set `self.StressValue` (+ (`self.StressIncreaseValue`) (`self.StressValue`))))
  (if (< 0.0 _output_get)
    (bind _outvector (`self.CalculateRandomEntitySpawnPosition` (`self.K2_GetActorLocation` (`GameplayStatics.GetPlayerPawn` 0))))
    (set `self.CalculatedSpawnVector` _outvector)
    (`self.SpawnEntities` 1)))

(event `SpawnEntities`
  (params (NbEntities :type Integer))
  (bind _calculatedspawnvector (`self.CalculatedSpawnVector`))
  (bind (_outitem _outindex) (`KismetArrayLibrary.Array_Random` (`self.list`)))
  (bind _output (`|GetArrayItem` (`self.StaticMeshList`) (`self.Index`)))
  (for _ (range (+ NbEntities 1))
    (set `self.Index` _outindex)
    (switch `/Game/EEntityList` _outitem
      (:`NewEnumerator0`
        (bind _returnvalue (`|SpawnActorFromClass` "/Game/BP_Entity.BP_Entity_C" (`KismetMathLibrary.MakeTransform` _calculatedspawnvector) "Undefined" "MultiplyWithRoot" null null))
        (`StaticMeshComponent.SetStaticMesh` (`/Game/BP_Entity.StaticMesh` _returnvalue) _output)
        (`KismetArrayLibrary.Array_Add` (`self.EntitiesSpawned`) _returnvalue)
        (`self.K2_SetActorRotation` _returnvalue (`KismetMathLibrary.FindLookAtRotation` (`self.K2_GetActorLocation` _returnvalue) (`self.K2_GetActorLocation` (`GameplayStatics.GetPlayerPawn` 0))) false)
        (`KismetSystemLibrary.PrintString` "entity spawned"))
      (:`NewEnumerator1`
        (bind _returnvalue_2 (`|SpawnActorFromClass` "/Game/BP_Entity.BP_Entity_C" (`KismetMathLibrary.MakeTransform` _calculatedspawnvector) "Undefined" "MultiplyWithRoot" null null))
        (`StaticMeshComponent.SetStaticMesh` (`/Game/BP_Entity.StaticMesh` _returnvalue_2) _output)
        (`KismetArrayLibrary.Array_Add` (`self.EntitiesSpawned`) _returnvalue_2))
      (:`NewEnumerator2`
        (bind _returnvalue_3 (`|SpawnActorFromClass` "/Game/BP_Entity.BP_Entity_C" (`KismetMathLibrary.MakeTransform` _calculatedspawnvector) "Undefined" "MultiplyWithRoot" null null))
        (`StaticMeshComponent.SetStaticMesh` (`/Game/BP_Entity.StaticMesh` _returnvalue_3) _output)
        (`KismetArrayLibrary.Array_Add` (`self.EntitiesSpawned`) _returnvalue_3)))))

(fn `CalculateRandomEntitySpawnPosition`
  (params (`actor location` :type "Vector Structure"))
  (returns (OutVector :type "Vector Structure"))
  (return (`KismetArrayLibrary.Array_Random` (`self.PossibleSpawnLocations`))))

(fn `ChangeStressLevel`
  (params (StressLevel :type Integer))
  (bind _output_get (set `self.StressLevel` StressLevel))
  (switch `int` _output_get
    (:`0`
      (for _array_element (`self.EntitiesSpawned`)
        (`self.K2_DestroyActor` _array_element)))
    (:`1`
      (for _array_element_2 (`self.EntitiesSpawned`)
        (`self.K2_DestroyActor` _array_element_2)))
    (:`2`
      (for _array_element_3 (`self.EntitiesSpawned`)
        (`self.K2_DestroyActor` _array_element_3)))
    (:`3`
      (for _array_element_4 (`self.EntitiesSpawned`)
        (`self.K2_DestroyActor` _array_element_4)))))

(fn `UserConstructionScript`)