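; Stress-system game mode (by name) that tracks a stress value, with events to raise or lower it across four threshold-based levels.
; Level changes call per-level functions: 0 clears entities and sets the player's point light, 1 is empty, 2 and 3 destroy entities.
; SpawnEntities places BP_Entity actors at random stored locations.
; Startup spawning, stress timer and mesh swaps are disconnected, and Tick's delayed sound switch never matches its constant input.
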(event `self.ReceiveBeginPlay`)

(event `SpawnEntities`
  (params (NbEntities :type Integer))
  (bind (_outitem _outindex) (`KismetArrayLibrary.Array_Random` (`self.list`)))
  (for _ (range (+ NbEntities 1))
    (set `self.Index` _outindex)
    (bind _outvector (`self.CalculateRandomEntitySpawnPosition` (`self.K2_GetActorLocation` (`GameplayStatics.GetPlayerPawn` 0))))
    (switch `/Game/Lucas/EEntityList` _outitem
      (:`NewEnumerator0`
        (bind _returnvalue (`|SpawnActorFromClass` "/Game/Lucas/BP_Entity.BP_Entity_C" (`KismetMathLibrary.MakeTransform` _outvector) "Undefined" "MultiplyWithRoot" null null))
        (`KismetArrayLibrary.Array_Add` (`self.EntitiesSpawned`) _returnvalue)
        (`self.K2_SetActorRotation` _returnvalue (`KismetMathLibrary.FindLookAtRotation` (`self.K2_GetActorLocation` _returnvalue) (`self.K2_GetActorLocation` (`GameplayStatics.GetPlayerPawn` 0))) false)
        (`KismetSystemLibrary.PrintString` "entity spawned"))
      (:`NewEnumerator1`
        (bind _returnvalue_2 (`|SpawnActorFromClass` "/Game/Lucas/BP_Entity.BP_Entity_C" (`KismetMathLibrary.MakeTransform` _outvector) "Undefined" "MultiplyWithRoot" null null))
        (`KismetArrayLibrary.Array_Add` (`self.EntitiesSpawned`) _returnvalue_2))
      (:`NewEnumerator2`
        (bind _returnvalue_3 (`|SpawnActorFromClass` "/Game/Lucas/BP_Entity.BP_Entity_C" (`KismetMathLibrary.MakeTransform` _outvector) "Undefined" "MultiplyWithRoot" null null))
        (`KismetArrayLibrary.Array_Add` (`self.EntitiesSpawned`) _returnvalue_3)))))

(event `IncreaseStress`
  (bind _output_get (set `self.StressValue` (+ (`self.StressIncreaseValue`) (`self.StressValue`))))
  (`KismetSystemLibrary.PrintString` (`KismetStringLibrary.Conv_DoubleToString` _output_get) true true (struct :`R` 1.0 :`B` 0.12597 :`A` 1.0) 2.0 "stress")
  (if (>= _output_get 30.0)
    (`KismetSystemLibrary.PrintString` "level 3" true true (struct :`G` 0.66 :`B` 1.0 :`A` 1.0) 2.0 "level")
    (`self.ChangeStressLevel` 3)
    (elif (>= _output_get 20.0)
      (`KismetSystemLibrary.PrintString` "level 2" true true (struct :`G` 0.66 :`B` 1.0 :`A` 1.0) 2.0 "level")
      (`self.ChangeStressLevel` 2)
      (elif (>= _output_get 10.0)
        (`KismetSystemLibrary.PrintString` "level 1" true true (struct :`G` 0.66 :`B` 1.0 :`A` 1.0) 2.0 "level")
        (`self.ChangeStressLevel` 1)
        (else
          (`KismetSystemLibrary.PrintString` "level 0" true true (struct :`G` 0.66 :`B` 1.0 :`A` 1.0) 2.0 "level")
          (`self.ChangeStressLevel` 0))))))

(event `DecreaseStress`
  (bind _output_get (set `self.StressValue` (- (`self.StressValue`) (`self.StressDecreaseValue`))))
  (`KismetSystemLibrary.PrintString` (`KismetStringLibrary.Conv_DoubleToString` _output_get) true true (struct :`R` 1.0 :`B` 0.12597 :`A` 1.0) 2.0 "stress")
  (if (< _output_get 30.0)
    (if (< _output_get 20.0)
      (if (< _output_get 10.0)
        (`KismetSystemLibrary.PrintString` "level 0" true true (struct :`G` 0.66 :`B` 1.0 :`A` 1.0) 2.0 "level")
        (`self.ChangeStressLevel` 0)
        (else
          (`KismetSystemLibrary.PrintString` "level 1" true true (struct :`G` 0.66 :`B` 1.0 :`A` 1.0) 2.0 "level")
          (`self.ChangeStressLevel` 1)))
      (else
        (`KismetSystemLibrary.PrintString` "level 2" true true (struct :`G` 0.66 :`B` 1.0 :`A` 1.0) 2.0 "level")
        (`self.ChangeStressLevel` 2)))
    (else
      (`KismetSystemLibrary.PrintString` "level 3" true true (struct :`G` 0.66 :`B` 1.0 :`A` 1.0) 2.0 "level")
      (`self.ChangeStressLevel` 3))))

(event `self.ReceiveTick`
  (params (DeltaSeconds :type "Float (single-precision)"))
  (`KismetSystemLibrary.Delay` (`KismetMathLibrary.RandomFloatInRange` 5.0 20.0))
  (switch `int` 0
    (:`1`
      (`GameplayStatics.PlaySound2D` "/Game/SoundDesign/stress2.stress2" 1.0 1.0 0.0 null null))
    (:`2`
      (`GameplayStatics.PlaySound2D` "/Game/SoundDesign/stress3.stress3" 1.0 1.0 0.0 null null))
    (:`3`
      (`GameplayStatics.PlaySound2D` "/Game/SoundDesign/stress4.stress4" 1.0 1.0 0.0 null null))))

(fn `CalculateRandomEntitySpawnPosition`
  (params (`actor location` :type "Vector Structure"))
  (returns (OutVector :type "Vector Structure"))
  (return (`KismetArrayLibrary.Array_Random` (`self.PossibleSpawnLocations`))))

(fn `ChangeStressLevel`
  (params (StressLevel :type Integer))
  (bind _entitiesspawned (`self.EntitiesSpawned`))
  (bind _returnvalue (`self.GetComponentByClass` (`GameplayStatics.GetPlayerPawn` 0) "/Script/Engine.PointLightComponent"))
  (if (not (== StressLevel (`self.StressLevel`)))
    (bind _output_get (set `self.StressLevel` StressLevel))
    (switch `int` _output_get
      (:`0`
        (if (!= (`KismetArrayLibrary.Array_Length` (`self.EntitiesSpawned`)) 0)
          (for (_array_element _array_index) _entitiesspawned
            (`KismetArrayLibrary.Array_Remove` _entitiesspawned _array_index)
            (`self.K2_DestroyActor` _array_element)
            (`LightComponent.SetIntensity` _returnvalue 80000.0 :!label _label)
            (`LocalLightComponent.SetAttenuationRadius` _returnvalue 5500.0))
          (else
            (goto _label))))
      (:`2`
        (for _array_element_2 (`self.EntitiesSpawned`)
          (`self.K2_DestroyActor` _array_element_2)))
      (:`3`
        (for _array_element_3 (`self.EntitiesSpawned`)
          (`self.K2_DestroyActor` _array_element_3))))))

(fn `UserConstructionScript`)